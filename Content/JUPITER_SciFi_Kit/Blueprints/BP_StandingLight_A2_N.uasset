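; Configurable standing light prop for the sci-fi kit, set up entirely in the construction script with no active runtime logic.
; Exposed variables pitch the rotating head, toggle the second lamp mesh and drive the RectLight's intensity, radius, color and mobility.
; A dynamic material instance matches the lamp glow to the light, with optional flickering through a light function.
; Switched-off or zero-intensity lights use the off material.
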(fn `UserConstructionScript`
  (bind _rectlight (`self.RectLight`))
  (bind _intensity (`self.Intensity`))
  (bind _flickering (`self.Flickering`))
  (bind _color (`self.Color`))
  (bind _mi_temporarylight (`self.MI_TemporaryLight`))
  (bind _rotatingpart (`self.RotatingPart`))
  ;[1 1 1] Change RotationParts Rotation
  (bind _output_get (set `self.InitRotation_RotatingPart` (`SceneComponent.RelativeRotation` _rotatingpart)))
  (`SceneComponent.K2_SetRelativeRotation` _rotatingpart (`KismetMathLibrary.MakeRotator` (.roll _output_get) (+ (.pitch _output_get) (`self.Rotation`)) (.yaw _output_get)) false false)
  ;[1 1 1] Hide One Mesh Part
  (`SceneComponent.SetVisibility` (`self.SM_StandingLight_A1_RotatingPart_N1`) (`self.One/Two_Lights`) false)
  ;[1 1 1] Light On/Off Toggle
  (if (`self.On/Off`)
    ;[1 1 1] Set RectLight Parameters
    (`LightComponent.SetIntensity` _rectlight _intensity)
    (`LocalLightComponent.SetAttenuationRadius` _rectlight (`self.Radius`))
    (`LightComponent.SetLightColor` _rectlight _color true)
    (`SceneComponent.SetMobility` _rectlight (`self.Type`))
    (if (<= _intensity 0.0)
      ;[1 1 1] Change Material If Light Is Off
      (`PrimitiveComponent.SetMaterial` (`self.SM_StandingLight_A1_RotatingPart_N`) 1 "/Game/JUPITER_SciFi_Kit/Materials/MI_Light_Off.MI_Light_Off" :!label _label)
      (`PrimitiveComponent.SetMaterial` (`self.SM_StandingLight_A1_RotatingPart_N1`) 1 "/Game/JUPITER_SciFi_Kit/Materials/MI_Light_Off.MI_Light_Off")
      (else
        ;[1 1 1] Set Light Material Parameters
        (bind _returnvalue (`KismetMaterialLibrary.CreateDynamicMaterialInstance` "/Game/JUPITER_SciFi_Kit/Materials/MI_Light_Warm.MI_Light_Warm"))
        (set `self.MI_TemporaryLight` _returnvalue)
        (`MaterialInstanceDynamic.SetVectorParameterValue` _mi_temporarylight "Light_Color" _color)
        (`MaterialInstanceDynamic.SetScalarParameterValue` _mi_temporarylight "Light_Intencity" (/ _intensity 1500.0))
        (`PrimitiveComponent.SetMaterial` (`self.SM_StandingLight_A1_RotatingPart_N`) 1 _mi_temporarylight)
        (`PrimitiveComponent.SetMaterial` (`self.SM_StandingLight_A1_RotatingPart_N1`) 1 _mi_temporarylight)
        ;[1 1 1] Flickering On/Off Toggle
        (if _flickering
          (`LightComponent.SetLightFunctionMaterial` (`self.RectLight`) "/Game/JUPITER_SciFi_Kit/Materials/M_Light_Flickering.M_Light_Flickering")
          (`MaterialInstanceDynamic.SetScalarParameterValue` (`self.MI_TemporaryLight`) "Flickering" (`KismetMathLibrary.Conv_BoolToDouble` _flickering)))))
    (else
      (`LightComponent.SetIntensity` _rectlight 0.0)
      (goto _label))))