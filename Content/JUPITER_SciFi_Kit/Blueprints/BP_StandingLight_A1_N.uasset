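; BP_StandingLight_A1_N is a configurable sci-fi standing light prop, set up entirely in the Construction Script with no active runtime logic.
; Height offsets the moving part, and Rotation pitches both rotating parts.
; When on, the RectLight takes the exposed settings, and a dynamic material matches its color and intensity, with optional flicker via light function and material parameter.
; Switching off or non-positive intensity applies an unlit lamp material.
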(fn `UserConstructionScript`
  (bind _rectlight (`self.RectLight`))
  (bind _rotatingpart_2 (`self.RotatingPart_2`))
  (bind _movingpart (`self.MovingPart`))
  (bind _intensity (`self.Intensity`))
  (bind _flickering (`self.Flickering`))
  (bind _color (`self.Color`))
  (bind _mi_temporarylight (`self.MI_TemporaryLight`))
  (bind _rotatingpart_1 (`self.RotatingPart_1`))
  (bind _rotation (`self.Rotation`))
  ;[1 1 1] Change MovingPart Height
  (bind _output_get (set `self.InitLocationMovingPart` (`SceneComponent.RelativeLocation` _movingpart)))
  (`SceneComponent.K2_SetRelativeLocation` _movingpart (`KismetMathLibrary.MakeVector` (.x _output_get) (.y _output_get) (+ (.z _output_get) (`self.Height`))) false false)
  ;[1 1 1] Change RotationParts Rotation
  (bind _output_get_2 (set `self.InitRotationRotatingPart1` (`SceneComponent.RelativeRotation` _rotatingpart_1)))
  (`SceneComponent.K2_SetRelativeRotation` _rotatingpart_1 (`KismetMathLibrary.MakeRotator` (.roll _output_get_2) (+ (.pitch _output_get_2) _rotation) (.yaw _output_get_2)) false false)
  (bind _output_get_3 (set `self.InitRotationRotatingPart2` (`SceneComponent.RelativeRotation` _rotatingpart_2)))
  (`SceneComponent.K2_SetRelativeRotation` _rotatingpart_2 (`KismetMathLibrary.MakeRotator` (.roll _output_get_3) (+ (.pitch _output_get_3) _rotation) (.yaw _output_get_3)) false false)
  ;[1 1 1] Light On/Off Toggle
  (if (`self.On/Off`)
    ;[1 1 1] Set RectLight Parameters
    (`LightComponent.SetIntensity` _rectlight _intensity)
    (`LocalLightComponent.SetAttenuationRadius` _rectlight (`self.Radius`))
    (`LightComponent.SetLightColor` _rectlight _color true)
    (`SceneComponent.SetMobility` _rectlight (`self.Type`))
    (if (<= _intensity 0.0)
      ;[1 1 1] Change Material If Light Is Off
      (`PrimitiveComponent.SetMaterial` (`self.SM_StandingLight_A1_RotatingPart_N`) 1 "/Game/JUPITER_SciFi_Kit/Materials/MI_Light_Off.MI_Light_Off" :!label _label)
      (`PrimitiveComponent.SetMaterial` (`self.SM_StandingLight_A1_RotatingPart_N1`) 1 "/Game/JUPITER_SciFi_Kit/Materials/MI_Light_Off.MI_Light_Off")
      (`PrimitiveComponent.SetMaterial` (`self.SM_StandingLight_A1_RotatingPart_N3`) 1 "/Game/JUPITER_SciFi_Kit/Materials/MI_Light_Off.MI_Light_Off")
      (`PrimitiveComponent.SetMaterial` (`self.SM_StandingLight_A1_RotatingPart_N2`) 1 "/Game/JUPITER_SciFi_Kit/Materials/MI_Light_Off.MI_Light_Off")
      (else
        ;[1 1 1] Set Light Material Parameters
        (bind _returnvalue (`KismetMaterialLibrary.CreateDynamicMaterialInstance` "/Game/JUPITER_SciFi_Kit/Materials/MI_Light_Warm.MI_Light_Warm"))
        (set `self.MI_TemporaryLight` _returnvalue)
        (`MaterialInstanceDynamic.SetVectorParameterValue` _mi_temporarylight "Light_Color" _color)
        (`MaterialInstanceDynamic.SetScalarParameterValue` _mi_temporarylight "Light_Intencity" (/ _intensity 1500.0))
        (`PrimitiveComponent.SetMaterial` (`self.SM_StandingLight_A1_RotatingPart_N`) 1 _mi_temporarylight)
        (`PrimitiveComponent.SetMaterial` (`self.SM_StandingLight_A1_RotatingPart_N1`) 1 _mi_temporarylight)
        (`PrimitiveComponent.SetMaterial` (`self.SM_StandingLight_A1_RotatingPart_N2`) 1 _mi_temporarylight)
        (`PrimitiveComponent.SetMaterial` (`self.SM_StandingLight_A1_RotatingPart_N3`) 1 _mi_temporarylight)
        ;[1 1 1] Flickering On/Off Toggle
        (if _flickering
          (`LightComponent.SetLightFunctionMaterial` (`self.RectLight`) "/Game/JUPITER_SciFi_Kit/Materials/M_Light_Flickering.M_Light_Flickering")
          (`MaterialInstanceDynamic.SetScalarParameterValue` (`self.MI_TemporaryLight`) "Flickering" (`KismetMathLibrary.Conv_BoolToDouble` _flickering)))))
    (else
      (`LightComponent.SetIntensity` _rectlight 0.0)
      (goto _label))))