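; Sci-fi kit door Blueprint that slides open when something enters its trigger volume and closes when it leaves.
; Trigger overlaps only set want-open and want-close flags, which a looping half-second timer polls, acting only while the door is not moving.
; A single timeline drives both directions, played forward or reversed, offsetting the Door component along relative Y from its initial location, scaled by DoorOpenLimit.
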(event `self.ReceiveBeginPlay`
  ;[1 1 1] Main door state flag:
  ; True = door Open
  ; False = door Closed
  (set `self.IsDoorOpen` false)
  ;[1 1 1] Door Flags: WantClose - if player leave trigger volume.
  ; WantOpen - if player inside of trigger doors
  (set `self.WantDoorOpen` false)
  (set `self.WantDoorClose` false)
  (set `self.IsDoorInProgress` false)
  ;[1 1 1] Store initial door locations
  (set `self.InitDoorLocation` (`SceneComponent.RelativeLocation` (`self.Door`)))
  ;[0.3708 0.3656 1] Timer! Each 0,5 sec we will check a door flags by executing CheckDoors event
  (bind _returnvalue (`KismetSystemLibrary.K2_SetTimer` null "CheckDoor" 0.5 true))
  (bind _output_get (set `self.CheckDoorTimeHandle` _returnvalue))
  (`KismetSystemLibrary.K2_UnPauseTimerHandle` _output_get))

(event `CheckDoor`
  ;[0.3708 0.3656 1] Main logic. Check door state. Checking every 0.5 seconds.
  (if (`self.IsDoorInProgress`)
    _
    (elif (`self.WantDoorOpen`)
      ;;[1 1 1] Ensure that door closed then process to Open
      (if (not (`self.IsDoorOpen`))
        (set `self.WantDoorOpen` false)
        (`self.OpenDoor`))
      (elif (`self.WantDoorClose`)
        ;;[1 1 1] Ensure that door is opened then process to Close
        (if (`self.IsDoorOpen`)
          (set `self.WantDoorClose` false)
          (`self.CloseDoor`))))))

(event `OpenDoor`
  (bind (_initdoorlocation_x _initdoorlocation_y _initdoorlocation_z) (`KismetMathLibrary.BreakVector` (`self.InitDoorLocation`)))
  ;[1 1 1] Open/Close animtation. Just pick valuer from time line and set Z location for door halfs
  (set `self.IsDoorInProgress` true)
  ;;[1 0.03484 0.1445] Change door state
  (set `self.IsDoorOpen` true)
  (bind (_direction _newtrack_0) (`Timeline|Timeline_0` :!via `PlayFromStart` :!label _label)
    (:`Update`
      (`SceneComponent.K2_SetRelativeLocation` (`self.Door`) (`KismetMathLibrary.MakeVector` _initdoorlocation_x (+ (* _newtrack_0 (`self.DoorOpenLimit`)) _initdoorlocation_y) _initdoorlocation_z) false false))
    (:`Finished`
      (set `self.IsDoorInProgress` false))))

(event `CloseDoor`
  ;[1 1 1] Open/Close animtation. Just pick valuer from time line and set Z location for door halfs
  (set `self.IsDoorInProgress` true)
  ;;[1 0.03484 0.1445] Change door state
  (set `self.IsDoorOpen` false)
  (goto _label :!via `ReverseFromEnd`))

(event `self.Door_Trigger.OnComponentBeginOverlap`
  (params (OverlappedComponent :type "PrimitiveComponent Object Reference") (OtherActor :type "Actor Object Reference") (OtherComp :type "PrimitiveComponent Object Reference") (OtherBodyIndex :type Integer) (bFromSweep :type Boolean) (SweepResult :type "HitResult Structure (by ref)"))
  ;[1 1 1] Tigger overlapping. Set / reset door flags.
  (set `self.WantDoorOpen` true)
  (set `self.WantDoorClose` false))

(event `self.Door_Trigger.OnComponentEndOverlap`
  (params (OverlappedComponent :type "PrimitiveComponent Object Reference") (OtherActor :type "Actor Object Reference") (OtherComp :type "PrimitiveComponent Object Reference") (OtherBodyIndex :type Integer))
  ;[1 1 1] Tigger overlapping. Set / reset door flags.
  (set `self.WantDoorClose` true)
  (set `self.WantDoorOpen` false))

(fn `UserConstructionScript`)