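; BP_Cable_D1_N is a construction-script tool that builds a sci-fi cable along an editable spline.
; It adds one deformed spline mesh per segment, matched to point locations and tangents, with query-only collision.
; Optional support meshes repeat at a set spacing along the spline's length.
; A bool-driven rotator lerp makes supports either follow the full spline rotation or keep only its yaw, staying upright.
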(fn `UserConstructionScript`
  (bind _distance_b_t_support_meshes (`self.Distance b/t Support Meshes`))
  (bind _spline (`self.Spline`))
  (bind _spline_2 (`self.Spline`))
  ;[1 1 1] Create Cable Along The Spline
  (for _index (range (+ (- (`SplineComponent.GetNumberOfSplinePoints` _spline) 2) 1))
    (bind _returnvalue (`AddComponent|NODE_AddSplineMeshComponent-4`))
    (`StaticMeshComponent.SetStaticMesh` _returnvalue "/Game/JUPITER_SciFi_Kit/Meshes/SM_Cable_D1_N.SM_Cable_D1_N")
    (`SplineMeshComponent.SetForwardAxis` _returnvalue "X" true)
    (`SceneComponent.K2_AttachToComponent` _returnvalue _spline "None" "KeepRelative" "KeepRelative" "KeepRelative" true)
    (bind _returnvalue_2 (+ _index 1))
    (`SplineMeshComponent.SetStartAndEnd` _returnvalue (`SplineComponent.GetLocationAtSplinePoint` _spline _index "Local") (`SplineComponent.GetTangentAtSplinePoint` _spline _index "Local") (`SplineComponent.GetLocationAtSplinePoint` _spline _returnvalue_2 "Local") (`SplineComponent.GetTangentAtSplinePoint` _spline _returnvalue_2 "Local") true)
    (`PrimitiveComponent.SetCollisionEnabled` _returnvalue "QueryOnly"))
  (if (`self.Add Support Meshes`)
    ;[1 1 1] Add Support Parts
    (for _index_2 (range (+ (`.ReturnValue` (`KismetMathLibrary.FMod` (`SplineComponent.GetSplineLength` _spline_2) _distance_b_t_support_meshes)) 1))
      (bind _returnvalue_3 (* _index_2 _distance_b_t_support_meshes))
      (bind _returnvalue_4 (`AddComponent|NODE_AddSplineMeshComponent-3` :`RelativeTransform` (`KismetMathLibrary.MakeTransform` (`SplineComponent.GetLocationAtDistanceAlongSpline` _spline_2 _returnvalue_3 "Local") (struct) (0.05 1.0 1.0))))
      (`StaticMeshComponent.SetStaticMesh` _returnvalue_4 "/Game/JUPITER_SciFi_Kit/Meshes/SM_Cable_D1_Support_N.SM_Cable_D1_Support_N")
      (`SplineMeshComponent.SetForwardAxis` _returnvalue_4 "X" true)
      (bind _returnvalue_5 (`SplineComponent.GetRotationAtDistanceAlongSpline` _spline_2 _returnvalue_3 "Local"))
      (`SceneComponent.K2_SetRelativeRotation` _returnvalue_4 (`KismetMathLibrary.RLerp` _returnvalue_5 (`KismetMathLibrary.MakeRotator` 0.0 0.0 (.yaw _returnvalue_5)) (`KismetMathLibrary.Conv_BoolToDouble` (`self.Rotate Support Meshes`))) false false))))