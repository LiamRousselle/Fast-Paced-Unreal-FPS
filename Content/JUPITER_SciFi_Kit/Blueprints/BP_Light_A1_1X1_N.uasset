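; Configurable light fixture from the JUPITER SciFi Kit, pairing a static mesh with a RectLight, set up entirely in the Construction Script.
; Exposed-style settings drive the light's intensity, radius, color and mobility.
; A dynamic instance of the warm light material mirrors color and scaled intensity on the mesh, swapping to an off material when disabled or at zero intensity.
; Optional flickering applies a light function and matching material parameter.
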(fn `UserConstructionScript`
  (bind _rectlight (`self.RectLight`))
  (bind _intensity (`self.Intensity`))
  (bind _flickering (`self.Flickering`))
  (bind _color (`self.Color`))
  (bind _mi_temporarylight (`self.MI_TemporaryLight`))
  ;[1 1 1] Light On/Off Toggle
  (if (`self.On/Off`)
    ;[1 1 1] Set RectLight Parameters
    (`LightComponent.SetIntensity` _rectlight _intensity)
    (`LocalLightComponent.SetAttenuationRadius` _rectlight (`self.Radius`))
    (`LightComponent.SetLightColor` _rectlight _color true)
    (`SceneComponent.SetMobility` _rectlight (`self.Type`))
    (if (<= _intensity 0.0)
      ;[1 1 1] Change Material If Light Is Off
      (`PrimitiveComponent.SetMaterial` (`self.SM_Light_A1_1X1_N`) 0 "/Game/JUPITER_SciFi_Kit/Materials/MI_Light_Off.MI_Light_Off" :!label _label)
      (else
        ;[1 1 1] Set Light Material Parameters
        (bind _returnvalue (`KismetMaterialLibrary.CreateDynamicMaterialInstance` "/Game/JUPITER_SciFi_Kit/Materials/MI_Light_Warm.MI_Light_Warm"))
        (set `self.MI_TemporaryLight` _returnvalue)
        (`MaterialInstanceDynamic.SetVectorParameterValue` _mi_temporarylight "Light_Color" _color)
        (`MaterialInstanceDynamic.SetScalarParameterValue` _mi_temporarylight "Light_Intencity" (/ _intensity 500.0))
        (`PrimitiveComponent.SetMaterial` (`self.SM_Light_A1_1X1_N`) 0 _mi_temporarylight)
        ;[1 1 1] Flickering On/Off Toggle
        (if _flickering
          (`LightComponent.SetLightFunctionMaterial` (`self.RectLight`) "/Game/JUPITER_SciFi_Kit/Materials/M_Light_Flickering.M_Light_Flickering")
          (`MaterialInstanceDynamic.SetScalarParameterValue` (`self.MI_TemporaryLight`) "Flickering" (`KismetMathLibrary.Conv_BoolToDouble` _flickering)))))
    (else
      (`LightComponent.SetIntensity` _rectlight 0.0)
      (goto _label))))